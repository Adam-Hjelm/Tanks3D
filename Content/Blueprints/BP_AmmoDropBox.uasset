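; BP_AmmoDropBox is an ammo pickup that grants ammo for a random weapon when overlapped.
; On overlap it picks a random option, skipping the first two, from the weapon select combo box in player zero's AimHUD.
; It strips numbers from the option, passes the name to the overlapping actor through PickedUpAmmoMessage, then destroys itself.
; An unfinished pop-up text widget block is present but never runs.
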(event `self.ReceiveActorBeginOverlap`
  (params (OtherActor :type "Actor Object Reference"))
  (bind _asbph_hudmaster (cast `/Game/Blueprints/UI/BPH_HUDMaster` (`PlayerController.GetHUD` (`GameplayStatics.GetPlayerController` 0))))
  (bind _aimhud (`/Game/Blueprints/UI/BPH_HUDMaster.AimHUD` _asbph_hudmaster))
  (bind _weaponselectcombobox (`/Game/Blueprints/UI/WB_AimTankHUD.WeaponSelectComboBox` _aimhud))
  (bind _nonnumericstring (`/Game/Blueprints/UI/WB_AimTankHUD.Split Numbers From String` _aimhud (`ComboBoxString.GetOptionAtIndex` _weaponselectcombobox (`KismetMathLibrary.RandomIntegerInRange` 2 (- (`ComboBoxString.GetOptionCount` _weaponselectcombobox) 1)))))
  (message `/Game/Blueprints/Interfaces/BPI_PlayerTank.PickedUpAmmo` OtherActor _nonnumericstring)
  (`self.K2_DestroyActor`))

(fn `UserConstructionScript`)