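; Player controller that lets one player switch possession between the tank pawns in the level.
; On BeginPlay it gathers all WheeledVehicleTankPawn actors, assigns each BP_AbramsTank its array index as player number, then possesses the selected one with game-only input.
; SwitchCharacter cycles through the list with wraparound, possessing and notifying each new tank.
; RemoveTankfromPlaying drops a tank from the list with debug prints, and GetAllTanks returns the list.
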(event `self.ReceiveBeginPlay`
  ;[1 1 1] INIT
  (bind _outactors (`GameplayStatics.GetAllActorsOfClass` "/Script/Tanks3D.WheeledVehicleTankPawn"))
  (bind _output_get (set `self.AvailableTankCharacters` _outactors))
  (for (_array_element _array_index) _output_get
    (bind _asbp_abrams_tank (cast `/Game/Blueprints/Player/BP_AbramsTank` _array_element))
    (set `/Game/Blueprints/Player/BP_AbramsTank.PlayerNumberIndex` _array_index _asbp_abrams_tank))
  (bind _output (`|GetArrayItem` _output_get (`self.CurrentSelectedCharacterIndex`)))
  (`self.Possess` _output)
  (message `/Game/Blueprints/Interfaces/BPI_PlayerTank.OnSwitchedTo` _output)
  (`WidgetBlueprintLibrary.SetInputMode_GameOnly` self))

(event `/Game/Blueprints/Interfaces/BPI_TankCharacterController.SwitchCharacter`
  (bind _output (`|GetArrayItem` (`self.AvailableTankCharacters`) (`self.CurrentSelectedCharacterIndex`)))
  (if (>= (`self.CurrentSelectedCharacterIndex`) (- (`KismetArrayLibrary.Array_Length` (`self.AvailableTankCharacters`)) 1))
    (set `self.CurrentSelectedCharacterIndex` 0)
    (else
      (set `self.CurrentSelectedCharacterIndex` (+ (`self.CurrentSelectedCharacterIndex`) 1))))
  (`self.Possess` _output)
  (message `/Game/Blueprints/Interfaces/BPI_PlayerTank.OnSwitchedTo` _output))

(event `/Game/Blueprints/Interfaces/BPI_TankCharacterController.RemoveTankFromPlaying`
  (params (TankToDisable :type "WheeledVehicleTankPawn Object Reference"))
  (`KismetSystemLibrary.PrintString` "REMOVING CHARACTER")
  (bind _returnvalue (`KismetArrayLibrary.Array_RemoveItem` (`self.AvailableTankCharacters`) TankToDisable))
  (`KismetSystemLibrary.PrintString` (`KismetStringLibrary.Concat_StrStr` (`KismetStringLibrary.Conv_BoolToString` _returnvalue) " tank was removed")))

(fn `GetAllTanks`
  (returns (`All Players` :type "Array of WheeledVehicleTankPawn Object Reference"))
  (return (`self.AvailableTankCharacters`)))

(fn `UserConstructionScript`)