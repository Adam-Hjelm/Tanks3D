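; Builder tank shell that adds a sphere of voxel terrain at its impact point instead of exploding on impact.
; Its alternate impact effect sphere-traces at dig radius, lifts player tanks above the build zone and damages each newly hit actor once without knockback.
; A voxel world hit gets the sphere added once, guarded by a flag, and the shot destroy call follows.
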(event `self.ReceiveBeginPlay`
  (set `self.ExplodeOnImpact` false)
  (`parent.ReceiveBeginPlay`))

(event `/Game/Blueprints/Interfaces/BPI_TankShell.AlternateImpactEffect`
  (bind _impact_point (`self.Impact Point`))
  (`KismetSystemLibrary.PrintString` "builder alternate boom")
  ;[1 1 1] Checks if sphere equal to DigRadius hit voxel world or player vehicle
  (bind (_outhits _returnvalue) (`KismetSystemLibrary.SphereTraceMultiForObjects` :`Start` _impact_point :`End` _impact_point :`Radius` (`self.DigRadius`) :`ObjectTypes` (`self.ObjectTypesArray`) :`DrawDebugType` "ForDuration"))
  (if _returnvalue
    (for _array_element _outhits
      (bind (_bblockinghit _binitialoverlap _time _distance _location _impactpoint _normal _impactnormal _physmat _hitactor) (`GameplayStatics.BreakHitResult` _array_element))
      (if (not (`KismetArrayLibrary.Array_Contains` (`self.TracedPlayerObjectNames`) (`KismetSystemLibrary.GetDisplayName` _hitactor)))
        (`self.Teleport Out of Build Zone` _hitactor)
        (message `/Game/Blueprints/Interfaces/BPI_PlayerTank.DamageTank` _hitactor _impactpoint (`self.Damage`) 0.0)
        (`KismetArrayLibrary.Array_Add` (`self.TracedPlayerObjectNames`) (`KismetSystemLibrary.GetDisplayName` _hitactor)))
      ;[1 1 1] Destructible Terrain Logic
      (if (not (`self.DoneVoxelWorldPhysics`))
        ;;[1 1 1] Destroy Terrain In Sphere
        (bind _asvoxel_world (cast `VoxelWorld` _hitactor) ; TODO: Change to interface in future
          (:`then`
            (`KismetSystemLibrary.PrintString` "cast suceeded")
            (bind _output_get (set `self.As Voxel World` _asvoxel_world))
            (`VoxelSphereTools.AddSphere` _output_get (`self.Impact Point`) (`self.DigRadius`))
            (set `self.DoneVoxelWorldPhysics` true))
          (:`CastFailed`
            (`KismetSystemLibrary.PrintString` "cast failed")))
        (`self.OnDestroyTankShot` :!label _label)))
    (else
      (goto _label))))

(fn `Teleport Out of Build Zone`
  (params (`Teleport Target` :type "Actor Object Reference"))
  (bind (_returnvalue_location _returnvalue_rotation) (`KismetMathLibrary.BreakTransform` (`self.GetTransform` `Teleport Target`)))
  (if (`KismetSystemLibrary.DoesImplementInterface` `Teleport Target` "/Game/Blueprints/Interfaces/BPI_PlayerTank.BPI_PlayerTank_C")
    (`self.K2_TeleportTo` `Teleport Target` (+ _returnvalue_location (0.0 0.0 750.0)) _returnvalue_rotation)))

(fn `UserConstructionScript`
  (`parent.UserConstructionScript`))