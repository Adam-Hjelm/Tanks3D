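; Tank shell variant that acts as a timed flamethrower burst from player 0's tank gun rather than an impact explosive.
; On BeginPlay it disables impact explosion, then attaches the flame Niagara or particle effect and burst sound to the player mesh.
; A separate BP_FlamethrowerCollider actor is spawned and snapped to the gun socket.
; After a fixed delay, the shell destroys itself and the collider.
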(event `self.ReceiveBeginPlay`
  (set `self.ExplodeOnImpact` false)
  (`self.ActivateFlamethrower`)
  (`parent.ReceiveBeginPlay`))

(event `ActivateFlamethrower`
  (bind _player_mesh (message `/Game/Blueprints/Interfaces/BPI_PlayerTank.GetPlayerMesh` (`GameplayStatics.GetPlayerPawn` 0)))
  (`NiagaraFunctionLibrary.SpawnSystemAttached` "/Game/FX/FXS_FlameThrower.FXS_FlameThrower" _player_mesh "gun_1_jntSocket" (200.0 0.0 50.0) (struct) "KeepRelativeOffset" true)
  (bind _returnvalue (`|SpawnActorFromClass` "/Game/Blueprints/TankAmmo/BP_FlamethrowerCollider.BP_FlamethrowerCollider_C" (`SceneComponent.GetSocketTransform` _player_mesh "gun_1_jntSocket" "RTS_World") "Undefined" "OverrideRootScale" (`GameplayStatics.GetPlayerPawn` 0) null))
  (`self.K2_AttachToComponent` _returnvalue _player_mesh "gun_1_jntSocket" "SnapToTarget" "SnapToTarget" "SnapToTarget" true)
  (bind (_returnvalue_location _returnvalue_rotation) (`KismetMathLibrary.BreakTransform` (`SceneComponent.GetSocketTransform` _player_mesh "gun_1_jntSocket" "RTS_World")))
  (`GameplayStatics.SpawnSoundAttached` "/Game/Sounds/Flame/BetterFlameThrowerLongBurst.BetterFlameThrowerLongBurst" _player_mesh "None" _returnvalue_location _returnvalue_rotation "KeepRelativeOffset" true 1.0 1.0 0.0 "/Game/Sounds/Attenuations/Att_Explosion.Att_Explosion" null)
  (`KismetSystemLibrary.Delay` 4.2)
  (`self.K2_DestroyActor`)
  (`self.K2_DestroyActor` _returnvalue))

(event `self.ReceiveTick`
  (params (DeltaSeconds :type "Float (single-precision)")))

(fn `UserConstructionScript`
  (`parent.UserConstructionScript`))