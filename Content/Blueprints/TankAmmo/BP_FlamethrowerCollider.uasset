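; Flamethrower damage volume that periodically hurts an Abrams player tank caught inside its box collider.
; BeginPlay briefly collapses and re-expands the box so overlaps register when spawned inside a target.
; Overlap events track one non-owner tank, matched by display name.
; Tick starts a looping timer once, which sends damage through DamageTankMessage with a randomized burst sound while contact lasts; component hits only print debug names.
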(event `self.ReceiveBeginPlay`
  (bind _boxcollider (`self.BoxCollider`))
  ;[1 1 1] To make sure ActorBeginOverlap triggers when spawned already inside object
  (`BoxComponent.SetBoxExtent` _boxcollider (0.0 0.0 0.0) true)
  (`KismetSystemLibrary.Delay` 0.05)
  (`BoxComponent.SetBoxExtent` _boxcollider (300.0 100.0 50.0) true))

(event `self.ReceiveActorBeginOverlap`
  (params (OtherActor :type "Actor Object Reference"))
  ;[1 1 1] Checks if flamethrower collider is overlapping a player tank
  (if (== OtherActor (`self.GetOwner`))
    _
    (elif (`KismetStringLibrary.Contains` (`KismetSystemLibrary.GetDisplayName` OtherActor) "BP_AbramsTank")
      (set `self.PlayerColliding` OtherActor)
      (set `self.isCollidingWithPlayer` true))))

(event `self.ReceiveActorEndOverlap`
  (params (OtherActor :type "Actor Object Reference"))
  ;[1 1 1] Checks if flamethrower collider is overlapping a player tank
  (if (`self.isCollidingWithPlayer`)
    (if (== OtherActor (`self.PlayerColliding`))
      (set `self.isCollidingWithPlayer` false))))

(event `self.ReceiveTick`
  (params (DeltaSeconds :type "Float (single-precision)"))
  ;[1 1 1] If CollidingWithPlayer true, deals damage to currently colliding tank
  (if (`self.isCollidingWithPlayer`)
    (`/Engine/EditorBlueprintResources/StandardMacros.DoOnce` false
      (:`Completed`
        (`KismetSystemLibrary.K2_SetTimerDelegate` (delegate `Deal Damage`) 0.5 true)))))

(event `Deal Damage`
  (bind _returnvalue (`self.K2_GetActorLocation`))
  (bind _returnvalue_2 (`KismetMathLibrary.RandomFloatInRange` 0.8 1.0))
  ;[1 1 1] If CollidingWithPlayer true, deals damage to currently colliding tank
  (if (`self.isCollidingWithPlayer`)
    (message `/Game/Blueprints/Interfaces/BPI_PlayerTank.DamageTank` (`self.PlayerColliding`) _returnvalue 5)
    (`GameplayStatics.PlaySoundAtLocation` "/Game/Sounds/Flame/FireBurst.FireBurst" _returnvalue (struct) _returnvalue_2 _returnvalue_2 0.0 "/Game/Sounds/Attenuations/Att_Explosion.Att_Explosion" null null null) ; Implement fire dmg sfx
  ))

(event `self.BoxCollider.OnComponentHit`
  (params (HitComponent :type "PrimitiveComponent Object Reference") (OtherActor :type "Actor Object Reference") (OtherComp :type "PrimitiveComponent Object Reference") (NormalImpulse :type "Vector Structure") (Hit :type "HitResult Structure (by ref)"))
  (bind _returnvalue (`KismetSystemLibrary.GetDisplayName` HitComponent))
  (if (`KismetSystemLibrary.DoesImplementInterface` HitComponent "/Game/Blueprints/Interfaces/BPI_PlayerTank.BPI_PlayerTank_C")
    (`KismetSystemLibrary.PrintString` _returnvalue)
    (else
      (`KismetSystemLibrary.PrintString` _returnvalue))))

(fn `UserConstructionScript`)