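; BP_TankShell_Cluster is a tank shell that splits into cluster bomblets on impact instead of exploding.
; BeginPlay configures inherited shell settings for damage, dig radius and voxel destruction, and turns off explode-on-impact before calling the parent.
; The AlternateImpactEffect override spawns AmountOfClusterBombs BP_TankShell_MiniClusters just above the impact point with random horizontal offsets and rotations.
; It then calls OnDestroyTankShot and destroys the shell.
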(event `self.ReceiveBeginPlay`
  (set `self.ExplodeOnImpact` false)
  (set `self.DigRadius` 300.0)
  (set `self.Damage` 10)
  (set `self.useAdvancedVoxelDestruction` false)
  (`parent.ReceiveBeginPlay`))

(event `self.ReceiveTick`
  (params (DeltaSeconds :type "Float (single-precision)"))
  (`parent.ReceiveTick` DeltaSeconds))

(event `/Game/Blueprints/Interfaces/BPI_TankShell.AlternateImpactEffect`
  (bind _returnvalue (`KismetMathLibrary.RandomFloatInRange` -50.0 50.0))
  (for _ (range 1 (+ (`self.AmountOfClusterBombs`) 1))
    (`|SpawnActorFromClass` "/Game/Blueprints/TankAmmo/BP_TankShell_MiniClusters.BP_TankShell_MiniClusters_C" (`KismetMathLibrary.MakeTransform` (+ (`self.Impact Point`) (`KismetMathLibrary.MakeVector` _returnvalue _returnvalue 100.0)) (`KismetMathLibrary.MakeRotator` 0.0 (`KismetMathLibrary.RandomFloatInRange` 0.0 360.0) (`KismetMathLibrary.RandomFloatInRange` 0.0 360.0))) "AlwaysSpawn" "OverrideRootScale" null 2.0 null))
  (`self.OnDestroyTankShot`)
  (`self.K2_DestroyActor`))

(fn `UserConstructionScript`
  (`parent.UserConstructionScript`))