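; Dig laser tank shell, a child of a shell parent that supplies the explosion logic.
; It enables the special explosion flag at BeginPlay and calls DoExplosion when its collision sphere begins an overlap.
; The special explosion and hit handlers only print debug text, so no digging or laser behavior is implemented here.
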(event `self.ReceiveBeginPlay`
  (set `self.SpecialExplosionEffect` true)
  (`parent.ReceiveBeginPlay`))

(event `/Game/Blueprints/Interfaces/BPI_TankShell.SpecialExplosion`
  (`KismetSystemLibrary.PrintString` "special explode laser"))

(event `self.SphereCollision.OnComponentBeginOverlap`
  (params (OverlappedComponent :type "PrimitiveComponent Object Reference") (OtherActor :type "Actor Object Reference") (OtherComp :type "PrimitiveComponent Object Reference") (OtherBodyIndex :type Integer) (bFromSweep :type Boolean) (SweepResult :type "HitResult Structure (by ref)"))
  (`KismetSystemLibrary.PrintString` "overlapping")
  (`self.DoExplosion`))

(event `self.SphereCollision.OnComponentHit`
  (params (HitComponent :type "PrimitiveComponent Object Reference") (OtherActor :type "Actor Object Reference") (OtherComp :type "PrimitiveComponent Object Reference") (NormalImpulse :type "Vector Structure") (Hit :type "HitResult Structure (by ref)"))
  (`KismetSystemLibrary.PrintString` "hit!"))

(fn `UserConstructionScript`
  (`parent.UserConstructionScript`))