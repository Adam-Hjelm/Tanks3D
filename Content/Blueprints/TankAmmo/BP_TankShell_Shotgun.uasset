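; BP_TankShell_Shotgun is a tank shell variant that fires a spread of pellets when it spawns.
; On BeginPlay it sets its own damage, dig radius and effect size, disables advanced voxel destruction, spawns the pellets, then calls parent BeginPlay.
; Each pellet is a BP_TankShell_Shotgun_Pellet spawned at the shell's location with randomized rotation, using a wider yaw and roll spread than pitch.
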(event `self.ReceiveBeginPlay`
  (set `self.DigRadius` 250.0)
  (set `self.Damage` 5)
  (set `self.useAdvancedVoxelDestruction` false)
  (set `self.EffectsSize` 0.3)
  (`self.SpawnShotgunPellets`)
  (`parent.ReceiveBeginPlay`))

(event `SpawnShotgunPellets`
  (bind (_returnvalue_roll _returnvalue_pitch _returnvalue_yaw) (`KismetMathLibrary.BreakRotator` (`self.K2_GetActorRotation`)))
  (for _ (range 1 (+ (`self.AmountOfShotGunPellets`) 1))
    (`|SpawnActorFromClass` "/Game/Blueprints/TankAmmo/BP_TankShell_Shotgun_Pellet.BP_TankShell_Shotgun_Pellet_C" (`KismetMathLibrary.MakeTransform` (`self.K2_GetActorLocation`) (`KismetMathLibrary.MakeRotator` (+ (`KismetMathLibrary.RandomFloatInRange` -25.0 25.0) _returnvalue_roll) (+ _returnvalue_pitch (`KismetMathLibrary.RandomFloatInRange` -10.0 10.0)) (+ _returnvalue_yaw (`KismetMathLibrary.RandomFloatInRange` -25.0 25.0)))) "AlwaysSpawn" "OverrideRootScale" null null)))

(fn `UserConstructionScript`
  (`parent.UserConstructionScript`))