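; Burrower tank shell Blueprint, kept in an Unused folder, that overrides the special explosion behavior of its parent shell.
; BeginPlay turns on the SpecialExplosionEffect flag before running the parent logic.
; SpecialExplosion sets the projectile velocity to the collision sphere's unscaled forward vector, slowing it to near standstill, and prints a debug string.
; No burrowing logic beyond that velocity change is implemented here.
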(event `self.ReceiveBeginPlay`
  (set `self.SpecialExplosionEffect` true)
  (`parent.ReceiveBeginPlay`))

(event `/Game/Blueprints/Interfaces/BPI_TankShell.SpecialExplosion`
  (set `MovementComponent.Velocity` (`SceneComponent.GetForwardVector` (`self.SphereCollision`)) (`self.ProjectileMovement`))
  (`KismetSystemLibrary.PrintString` "1"))

(fn `UserConstructionScript`
  (`parent.UserConstructionScript`))