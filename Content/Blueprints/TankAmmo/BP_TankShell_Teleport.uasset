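; BP_TankShell_Teleport is a tank shell variant that teleports the player's pawn to where it lands.
; On BeginPlay it turns off ExplodeOnImpact before calling the parent shell logic.
; Its AlternateImpactEffect moves player 0's pawn just above the impact point keeping its rotation, prints the result, spawns a magic burst Niagara effect there, then calls OnDestroyTankShot.
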(event `self.ReceiveBeginPlay`
  (set `self.ExplodeOnImpact` false)
  (`parent.ReceiveBeginPlay`))

(event `/Game/Blueprints/Interfaces/BPI_TankShell.AlternateImpactEffect`
  (bind _returnvalue (`Controller.K2_GetPawn` (`GameplayStatics.GetPlayerController` 0)))
  (bind _returnvalue_2 (`self.K2_TeleportTo` _returnvalue (+ (`self.Impact Point`) (0.0 0.0 200.0)) (`self.K2_GetActorRotation` _returnvalue)))
  (`KismetSystemLibrary.PrintString` (`KismetStringLibrary.Conv_BoolToString` _returnvalue_2))
  (`NiagaraFunctionLibrary.SpawnSystemAtLocation` "/Game/FX/NS_MagicBurst.NS_MagicBurst" (+ (`self.Impact Point`) (0.0 0.0 200.0)) (struct) (5.0 5.0 5.0))
  (`self.OnDestroyTankShot`))

(fn `UserConstructionScript`
  (`parent.UserConstructionScript`))