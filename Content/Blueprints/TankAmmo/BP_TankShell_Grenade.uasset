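; Tank shell variant that acts as a timed grenade, with impact detonation switched off and its own damage value.
; On BeginPlay it attaches a looping-style beep cue to the sphere mesh, stopping when the shell is destroyed.
; Tick feeds the shell's age into the cue's BeepPitch parameter and calls DoExplosion once it passes five seconds.
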(event `self.ReceiveBeginPlay`
  (set `self.ExplodeOnImpact` false)
  (bind _returnvalue (`GameplayStatics.SpawnSoundAttached` "/Game/Sounds/ExplosiveBeepSound_Cue.ExplosiveBeepSound_Cue" (`self.SphereStaticMesh`) "None" (0.0 0.0 0.0) (struct) "KeepRelativeOffset" true 1.0 1.0 0.0 null null))
  (set `self.BeepSound` _returnvalue)
  (set `self.Damage` 50)
  (`parent.ReceiveBeginPlay`))

(event `self.ReceiveTick`
  (params (DeltaSeconds :type "Float (single-precision)"))
  (`AudioParameterControllerInterface.SetFloatParameter` (`self.BeepSound`) "BeepPitch" (`self.Lifetime`))
  (bind _output_get (set `self.Lifetime` (`self.GetGameTimeSinceCreation`)))
  (if (> _output_get 5.0)
    (`self.DoExplosion`))
  (`parent.ReceiveTick` DeltaSeconds))

(fn `UserConstructionScript`
  (`parent.UserConstructionScript`))